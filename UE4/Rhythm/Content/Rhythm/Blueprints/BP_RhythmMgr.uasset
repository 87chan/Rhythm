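; Rhythm manager for a two-player call-and-response duel where one player performs a beat pattern and the other traces it.
; A looping BPM timer drives the countdown, metronome and turn cycle through both players' perform and trace phases.
; Inputs mark beat slots by matching Tick-accumulated time against threshold windows.
; After each trace the two lists are compared, and a mismatch announces the winner and pauses the game.
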(event Custom|OnUpdate
  (bind _progress (Variables|Default|GetProgress))
  (bind _bpmcounter (Variables|Default|GetBPMCounter))
  (bind _phrase (Variables|Default|GetPhrase))
  (bind _phraseinterval (Variables|Default|GetPhraseInterval))
  (bind _returnvalue (* _phrase _phraseinterval))
  (bind _returnvalue_2 (Math|Integer|%(Integer) _bpmcounter _returnvalue))
  (Utilities|FlowControl|Sequence
    (:then_0
      (if (and (or (Utilities|Enum|Equal(Enum) _progress "NewEnumerator2") (Utilities|Enum|Equal(Enum) _progress "NewEnumerator4")) (CallFunction|CheckGameStart))
        (if (Utilities|Enum|NotEqual(Enum) (Utilities|Array|Get(acopy) (Variables|Default|GetBeatListPerform) _returnvalue_2) (Utilities|Array|Get(acopy) (Variables|Default|GetBeatListTrace) _returnvalue_2))
          (Utilities|Array|Add (Variables|Default|GetBeatListMiss) _returnvalue_2)
          (Development|PrintString "Hello"))))
    (:then_1
      (bind _result (Math|Integer|IncrementInt (Variables|Default|GetBPMCounter))
        (:%20%20
          (if (== (Math|Integer|%(Integer) _result (Variables|Default|GetPhrase)) 0)
            (bind _result_2 (Math|Integer|IncrementInt (Variables|Default|GetPhraseCounter))
              (:%20%20
                (if (>= _result_2 0)
                  (Utilities|FlowControl|Sequence
                    (:then_0
                      (if (== (Math|Integer|%(Integer) _result_2 (Variables|Default|GetPhraseInterval)) 0)
                        (Utilities|FlowControl|Sequence
                          (:then_0
                            (CallFunction|NextProgress)
                            (switch Utilities|FlowControl|Switch|SwitchonEProgress (Variables|Default|GetProgress)
                              (:NewEnumerator1
                                (if (CallFunction|IsEqual (Variables|Default|GetBeatListPerform) (Variables|Default|GetBeatListTrace)) :!label _label
                                  (CallFunction|ResetBeatList (Variables|Default|GetBeatListPerform))
                                  (CallFunction|ResetBeatList (Variables|Default|GetBeatListTrace))
                                  (Utilities|Array|Clear (Variables|Default|GetBeatListMiss))
                                  (else
                                    (Variables|Default|SetIsGameEnd true))))
                              (:NewEnumerator2
                                (CallFunction|ResetBeatList (Variables|Default|GetBeatListTrace) :!label _label_2))
                              (:NewEnumerator3
                                (goto _label))
                              (:NewEnumerator4
                                (goto _label_2))))
                          (:then_1
                            (if (Variables|Default|GetIsGameEnd)
                              (switch Utilities|FlowControl|Switch|SwitchonEProgress (Variables|Default|GetProgress)
                                (:NewEnumerator1
                                  (Development|PrintString "2P Win!"))
                                (:NewEnumerator3
                                  (Development|PrintString "1P Win!")))
                              (Audio|PlaySound2D "/Game/Rhythm/Sounds/Onmtp-Ding.Onmtp-Ding")
                              (Game|SetGamePaused true)
                              (else
                                (switch Utilities|FlowControl|Switch|SwitchonEProgress (Variables|Default|GetProgress)
                                  (:NewEnumerator1
                                    (CallFunction|On1PPerform))
                                  (:NewEnumerator2
                                    (CallFunction|On2PTrace))
                                  (:NewEnumerator3
                                    (CallFunction|On2PPerform))
                                  (:NewEnumerator4
                                    (CallFunction|On1PTrace)))))))))
                    (:then_1
                      (if (not (Variables|Default|GetIsGameEnd))
                        (Audio|PlaySound2D "/Game/Rhythm/Sounds/wood-block.wood-block"))))
                  (else
                    (switch int (* (Variables|Default|GetPhraseCounter) -1)
                      (:1
                        (Development|PrintString "Start!!" true true "(R=0.000000,G=0.660000,B=1.000000,A=1.000000)" 0.5)
                        (Audio|PlaySound2D "/Game/Rhythm/Sounds/Onmtp-Ding.Onmtp-Ding"))
                      (:2
                        (Development|PrintString "1" true true "(R=0.000000,G=0.660000,B=1.000000,A=1.000000)" 0.5)
                        (Audio|PlaySound2D "/Game/Rhythm/Sounds/wood-block.wood-block" :!label _label_3))
                      (:3
                        (Development|PrintString "2" true true "(R=0.000000,G=0.660000,B=1.000000,A=1.000000)" 0.5)
                        (goto _label_3))
                      (:4
                        (Development|PrintString "3" true true "(R=0.000000,G=0.660000,B=1.000000,A=1.000000)" 0.5)
                        (goto _label_3)))))))))))))

(event Custom|On1PPerform
  (Development|PrintString "1P Perform" true true "(R=0.000000,G=0.660000,B=1.000000,A=1.000000)" 0.5)
  (Variables|Default|SetBPMCounter 0)
  (Variables|Default|SetTimeCounter 0.0))

(event Custom|On2PTrace
  (Development|PrintString "2P Trace" true true "(R=1.000000,G=0.000000,B=0.000000,A=1.000000)" 0.5)
  (Variables|Default|SetBPMCounter 0)
  (Variables|Default|SetTimeCounter 0.0))

(event Custom|On2PPerform
  (Development|PrintString "2P Perform" true true "(R=1.000000,G=0.000000,B=0.000000,A=1.000000)" 0.5)
  (Variables|Default|SetBPMCounter 0)
  (Variables|Default|SetTimeCounter 0.0))

(event Custom|On1PTrace
  (Development|PrintString "1P Trace" true true "(R=0.000000,G=0.660000,B=1.000000,A=1.000000)" 0.5)
  (Variables|Default|SetBPMCounter 0)
  (Variables|Default|SetTimeCounter 0.0))

(event EventBeginPlay
  (Variables|Default|SetPhraseCounter (- (Variables|Default|GetPhraseCounter) (Variables|Default|GetBeginPhrase)))
  (Utilities|Time|SetTimerbyEvent (delegate Custom|OnUpdate) (/ 1.0 (/ (Math|Conversions|ToFloat(Integer) (Variables|Default|GetBPM)) 6e+01)) true))

(event EventTick
  (params (DeltaSeconds :type Float%20%28single-precision%29))
  (Variables|Default|SetTimeCounter (+ (Variables|Default|GetTimeCounter) DeltaSeconds)))

(event Input|ActionEvents|InputActionRightBeat_1P
  (params (Key :type Key%20Structure))
  (:Pressed
    (Utilities|GameStart
      (:True
        (switch Utilities|FlowControl|Switch|SwitchonEProgress (Variables|Default|GetProgress)
          (:NewEnumerator1
            (CallFunction|Beat (Variables|Default|GetBeatListPerform)))
          (:NewEnumerator4
            (CallFunction|Beat (Variables|Default|GetBeatListTrace))))))))

(event Input|ActionEvents|InputActionRightBeat_2P
  (params (Key :type Key%20Structure))
  (:Pressed
    (Utilities|GameStart
      (:True
        (switch Utilities|FlowControl|Switch|SwitchonEProgress (Variables|Default|GetProgress)
          (:NewEnumerator2
            (CallFunction|Beat (Variables|Default|GetBeatListTrace)))
          (:NewEnumerator3
            (CallFunction|Beat (Variables|Default|GetBeatListPerform))))))))

(event Input|ActionEvents|InputActionLeftBeat_1P
  (params (Key :type Key%20Structure))
  (:Pressed
    (Utilities|GameStart
      (:True
        (switch Utilities|FlowControl|Switch|SwitchonEProgress (Variables|Default|GetProgress)
          (:NewEnumerator1
            (CallFunction|Beat (Variables|Default|GetBeatListPerform)))
          (:NewEnumerator4
            (CallFunction|Beat (Variables|Default|GetBeatListTrace))))))))

(event Input|ActionEvents|InputActionLeftBeat_2P
  (params (Key :type Key%20Structure))
  (:Pressed
    (Utilities|GameStart
      (:True
        (switch Utilities|FlowControl|Switch|SwitchonEProgress (Variables|Default|GetProgress)
          (:NewEnumerator2
            (CallFunction|Beat (Variables|Default|GetBeatListTrace)))
          (:NewEnumerator3
            (CallFunction|Beat (Variables|Default|GetBeatListPerform))))))))

(fn ConstructionScript)

(fn NextProgress
  (Variables|Default|SetProgress (Utilities|Enum|ByteToEnumEProgress (Math|Conversions|ToByte(Integer) (Math|Integer|%(Integer) (+ (Math|Conversions|ToInteger(Byte) (Variables|Default|GetProgress)) 1) (Math|Conversions|ToInteger(Byte) (Utilities|Enum|LiteralenumEProgress "NewEnumerator5")))))))

(fn Beat
  (params (BeatList :type Array%20of%20EBeatType%20Enums :default "NewEnumerator0"))
  (bind _phraseinterval (Variables|Default|GetPhraseInterval))
  (bind _phrase (Variables|Default|GetPhrase))
  (bind _phraseinterval_2 (Variables|Default|GetPhraseInterval))
  (bind _effectivethreshould (Variables|Default|GetEffectiveThreshould))
  (bind _returnvalue (* _phrase _phraseinterval_2))
  (bind _returnvalue_2 (/ _returnvalue _phraseinterval))
  (bind _returnvalue_3 (Math|Conversions|ToFloat(Integer) _returnvalue_2))
  (bind _returnvalue_4 (/ 1.0 _returnvalue_3))
  (bind _returnvalue_5 (* _effectivethreshould _returnvalue_4))
  (for _index (range 0 (- _returnvalue 1))
    (if (Math|Float|InRange(Float) (Variables|Default|GetTimeCounter) (- (* _index _returnvalue_4) _returnvalue_5) (+ (* _index _returnvalue_4) _returnvalue_5))
      (Utilities|Array|SetArrayElem BeatList _index "NewEnumerator1")
      (Audio|PlaySound2D "/Game/Rhythm/Sounds/small_drum.small_drum"))))

(fn CheckGameStart
  (return (>= (Variables|Default|GetPhraseCounter) 0)))

(fn ResetBeatList
  (params (List :type Array%20of%20EBeatType%20Enums :default "NewEnumerator0"))
  (Utilities|Array|Clear List)
  (Utilities|Array|Resize List (* (Variables|Default|GetPhrase) (Variables|Default|GetPhraseInterval))))

(fn IsEqual
  (params (BeatListA :type Array%20of%20EBeatType%20Enums :default "NewEnumerator0") (BeatListB :type Array%20of%20EBeatType%20Enums :default "NewEnumerator0"))
  (bind _returnvalue (Utilities|Array|Length BeatListA))
  (if (== _returnvalue (Utilities|Array|Length BeatListB))
    (for _index (range 0 (- _returnvalue 1))
      (if (Utilities|Enum|NotEqual(Enum) (Utilities|Array|Get(acopy) BeatListB _index) (Utilities|Array|Get(acopy) BeatListA _index))
        (return false)))
    (return true)
    (else
      (return false))))