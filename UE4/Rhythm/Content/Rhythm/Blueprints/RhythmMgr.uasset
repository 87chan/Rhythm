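; Rhythm manager that paces a two-player turn-based call-and-response, with perform and trace phases.
; A looping timer derived from BPM and Phrase length plays a woodblock and advances a phrase counter, offset negative for a printed countdown.
; At each phrase interval, nested FlipFlops cycle 1P perform, 2P trace, 2P perform, 1P trace.
; The four phase events currently only print their names.
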(event Custom|OnUpdate
  (Audio|PlaySound2D "/Game/Rhythm/Sounds/wood-block.wood-block")
  (bind _result (Math|Integer|IncrementInt (Variables|Default|GetPhraseCounter))
    (:%20%20
      (if (and (>= _result 0) (== (Math|Integer|%(Integer) _result (Variables|Default|GetPhraseInterval)) 0))
        (Utilities|FlowControl|FlipFlop
          (:A
            (Utilities|FlowControl|FlipFlop
              (:A
                (CallFunction|On1PPerform))
              (:B
                (CallFunction|On2PPerform))))
          (:B
            (Utilities|FlowControl|FlipFlop
              (:A
                (CallFunction|On2PTrace))
              (:B
                (CallFunction|On1PTrace)))))
        (else
          (switch int (* (Variables|Default|GetPhraseCounter) -1)
            (:1
              (Development|PrintString "Start!!" true true "(R=0.000000,G=0.660000,B=1.000000,A=1.000000)" 0.5))
            (:2
              (Development|PrintString "1" true true "(R=0.000000,G=0.660000,B=1.000000,A=1.000000)" 0.5))
            (:3
              (Development|PrintString "2" true true "(R=0.000000,G=0.660000,B=1.000000,A=1.000000)" 0.5))
            (:4
              (Development|PrintString "3" true true "(R=0.000000,G=0.660000,B=1.000000,A=1.000000)" 0.5))))))))

(event Custom|On1PPerform
  (Development|PrintString "1P Perform" true true "(R=0.000000,G=0.660000,B=1.000000,A=1.000000)" 0.5))

(event Custom|On2PTrace
  (Development|PrintString "2P Trace" true true "(R=1.000000,G=0.000000,B=0.000000,A=1.000000)" 0.5))

(event Custom|On2PPerform
  (Development|PrintString "2P Perform" true true "(R=1.000000,G=0.000000,B=0.000000,A=1.000000)" 0.5))

(event Custom|On1PTrace
  (Development|PrintString "1P Trace" true true "(R=0.000000,G=0.660000,B=1.000000,A=1.000000)" 0.5))

(event EventBeginPlay
  (Variables|Default|SetPhraseCounter (- (Variables|Default|GetPhraseCounter) (Variables|Default|GetBeginPhrase)))
  (Utilities|Time|SetTimerbyEvent (delegate Custom|OnUpdate) (* (/ 1.0 (/ (Math|Conversions|ToFloat(Integer) (Variables|Default|GetBPM)) 6e+01)) (Math|Conversions|ToFloat(Integer) (Variables|Default|GetPhrase))) true))

(fn ConstructionScript)